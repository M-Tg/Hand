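; BP_box_1 is a physics box that tracks whether it can be grabbed, pushed, climbed or stood on.
; Seven overlap volumes set the state flags, and Tick re-toggles their collision to force fresh overlap checks.
; Tick also tints a dynamic material by state and, while grounded, disables physics if PlayerOn is overlapped.
; IsGrabedF switches gravity off when this box is the grabbed one.
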(event `self.ReceiveBeginPlay`)

(event `CollisionCheck`
  (params (Collision :type "PrimitiveComponent Object Reference"))
  (`PrimitiveComponent.SetCollisionEnabled` Collision "NoCollision")
  (`PrimitiveComponent.SetCollisionEnabled` Collision "QueryOnly"))

(event `self.ReceiveTick`
  (params (DeltaSeconds :type "Float (single-precision)"))
  (`self.CollisionCheck` (`self.PlayerOn`))
  (`self.CollisionCheck` (`self.Left`))
  (`self.CollisionCheck` (`self.Right`))
  (`self.CollisionCheck` (`self.Down`))
  (`self.CollisionCheck` (`self.Up`))
  (`self.CollisionCheck` (`self.UpLSide`))
  (`self.CollisionCheck` (`self.UpRSide`))
  (if (`self.Grounded`)
    (if (`self.Stamped`)
      (`PrimitiveComponent.SetSimulatePhysics` (`self.Cube`) false)
      (`MaterialInstanceDynamic.SetVectorParameterValue` (`self.CubeMaterial`) "SampleColor" (struct :`R` 0.540942 :`G` 0.021307 :`B` 0.869792 :`A` 1.0))
      (else
        (`PrimitiveComponent.SetSimulatePhysics` (`self.Cube`) true)
        (if (`self.CanBeGrabed`)
          (if (`self.CanBePushedR`)
            (if (`self.CanBePushedL`)
              (`MaterialInstanceDynamic.SetVectorParameterValue` (`self.CubeMaterial`) "SampleColor" (struct :`R` 0.283715 :`G` 0.797356 :`B` 0.916667 :`A` 1.0))
              (else
                (`MaterialInstanceDynamic.SetVectorParameterValue` (`self.CubeMaterial`) "SampleColor" (struct :`R` 0.25241 :`G` 0.916667 :`B` 0.212072 :`A` 1.0) :!label _label)))
            (else
              (goto _label)))
          (else
            (`MaterialInstanceDynamic.SetVectorParameterValue` (`self.CubeMaterial`) "SampleColor" (struct :`R` 0.916667 :`G` 0.131587 :`B` 0.186345 :`A` 1.0))))))
    (else
      (`MaterialInstanceDynamic.SetVectorParameterValue` (`self.CubeMaterial`) "SampleColor" (struct :`R` 0.916667 :`G` 0.754615 :`B` 0.139466 :`A` 1.0)))))

(event `self.PlayerOn.OnComponentBeginOverlap`
  (params (OverlappedComponent :type "PrimitiveComponent Object Reference") (OtherActor :type "Actor Object Reference") (OtherComp :type "PrimitiveComponent Object Reference") (OtherBodyIndex :type Integer) (bFromSweep :type Boolean) (SweepResult :type "HitResult Structure (by ref)"))
  (set `self.Stamped` true))

(event `self.PlayerOn.OnComponentEndOverlap`
  (params (OverlappedComponent :type "PrimitiveComponent Object Reference") (OtherActor :type "Actor Object Reference") (OtherComp :type "PrimitiveComponent Object Reference") (OtherBodyIndex :type Integer))
  (set `self.Stamped` false))

(event `self.UpLSide.OnComponentBeginOverlap`
  (params (OverlappedComponent :type "PrimitiveComponent Object Reference") (OtherActor :type "Actor Object Reference") (OtherComp :type "PrimitiveComponent Object Reference") (OtherBodyIndex :type Integer) (bFromSweep :type Boolean) (SweepResult :type "HitResult Structure (by ref)"))
  (set `self.CanBeClimbedL` false))

(event `self.Up.OnComponentBeginOverlap`
  (params (OverlappedComponent :type "PrimitiveComponent Object Reference") (OtherActor :type "Actor Object Reference") (OtherComp :type "PrimitiveComponent Object Reference") (OtherBodyIndex :type Integer) (bFromSweep :type Boolean) (SweepResult :type "HitResult Structure (by ref)"))
  (set `self.CanBeGrabed` false))

(event `self.UpRSide.OnComponentBeginOverlap`
  (params (OverlappedComponent :type "PrimitiveComponent Object Reference") (OtherActor :type "Actor Object Reference") (OtherComp :type "PrimitiveComponent Object Reference") (OtherBodyIndex :type Integer) (bFromSweep :type Boolean) (SweepResult :type "HitResult Structure (by ref)"))
  (set `self.CanBeClimbedR` false))

(event `self.UpLSide.OnComponentEndOverlap`
  (params (OverlappedComponent :type "PrimitiveComponent Object Reference") (OtherActor :type "Actor Object Reference") (OtherComp :type "PrimitiveComponent Object Reference") (OtherBodyIndex :type Integer))
  (set `self.CanBeClimbedL` true))

(event `self.Up.OnComponentEndOverlap`
  (params (OverlappedComponent :type "PrimitiveComponent Object Reference") (OtherActor :type "Actor Object Reference") (OtherComp :type "PrimitiveComponent Object Reference") (OtherBodyIndex :type Integer))
  (set `self.CanBeGrabed` true))

(event `self.UpRSide.OnComponentEndOverlap`
  (params (OverlappedComponent :type "PrimitiveComponent Object Reference") (OtherActor :type "Actor Object Reference") (OtherComp :type "PrimitiveComponent Object Reference") (OtherBodyIndex :type Integer))
  (set `self.CanBeClimbedR` true))

(event `self.Left.OnComponentBeginOverlap`
  (params (OverlappedComponent :type "PrimitiveComponent Object Reference") (OtherActor :type "Actor Object Reference") (OtherComp :type "PrimitiveComponent Object Reference") (OtherBodyIndex :type Integer) (bFromSweep :type Boolean) (SweepResult :type "HitResult Structure (by ref)"))
  (set `self.CanBePushedL` false))

(event `self.Right.OnComponentBeginOverlap`
  (params (OverlappedComponent :type "PrimitiveComponent Object Reference") (OtherActor :type "Actor Object Reference") (OtherComp :type "PrimitiveComponent Object Reference") (OtherBodyIndex :type Integer) (bFromSweep :type Boolean) (SweepResult :type "HitResult Structure (by ref)"))
  (set `self.CanBePushedR` false))

(event `self.Down.OnComponentBeginOverlap`
  (params (OverlappedComponent :type "PrimitiveComponent Object Reference") (OtherActor :type "Actor Object Reference") (OtherComp :type "PrimitiveComponent Object Reference") (OtherBodyIndex :type Integer) (bFromSweep :type Boolean) (SweepResult :type "HitResult Structure (by ref)"))
  (set `self.Grounded` true))

(event `self.Left.OnComponentEndOverlap`
  (params (OverlappedComponent :type "PrimitiveComponent Object Reference") (OtherActor :type "Actor Object Reference") (OtherComp :type "PrimitiveComponent Object Reference") (OtherBodyIndex :type Integer))
  (set `self.CanBePushedL` true))

(event `self.Right.OnComponentEndOverlap`
  (params (OverlappedComponent :type "PrimitiveComponent Object Reference") (OtherActor :type "Actor Object Reference") (OtherComp :type "PrimitiveComponent Object Reference") (OtherBodyIndex :type Integer))
  (set `self.CanBePushedR` true))

(event `self.Down.OnComponentEndOverlap`
  (params (OverlappedComponent :type "PrimitiveComponent Object Reference") (OtherActor :type "Actor Object Reference") (OtherComp :type "PrimitiveComponent Object Reference") (OtherBodyIndex :type Integer))
  (set `self.Grounded` false))

(fn `IsGrabed_F`
  (params (GrabedComp :type "PrimitiveComponent Object Reference"))
  (if (== GrabedComp "BP_box_1")
    (`PrimitiveComponent.SetEnableGravity` (`self.Cube`) false)
    (else
      (`PrimitiveComponent.SetEnableGravity` (`self.Cube`) true))))

(fn `UserConstructionScript`
  ;[1 1 1] マテリアルをダイナミックインスタンス化　選んだ親マテリアルをベースにメッシュ用のマテリアル作成
  (bind _returnvalue (`KismetMaterialLibrary.CreateDynamicMaterialInstance` "/Game/M/Hand/BP/BP_Objects/SampleMaterial.SampleMaterial" "SampleMaterial"))
  (bind _output_get (set `self.CubeMaterial` _returnvalue))
  (`PrimitiveComponent.SetMaterial` (`self.Cube`) 0 _output_get)
  (`MaterialInstanceDynamic.SetVectorParameterValue` _output_get "SampleColor" (struct :`R` 0.283715 :`G` 0.797356 :`B` 0.916667 :`A` 1.0)))