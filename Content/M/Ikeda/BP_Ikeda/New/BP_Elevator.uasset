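; BP_Elevator is an elevator that moves its Cube vertically while something overlaps the Box1 trigger.
; BeginPlay caches the Cube's start location, and a timeline adds its track value to that Z on each update.
; Begin overlap plays the timeline and end overlap stops it, halting the Cube mid-travel.
; An unfinished, unreached height check is noted as intended to carry it on to the top or bottom after early exit.
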(event `self.ReceiveBeginPlay`
  (bind _output_get (set `self.startPotision` (`SceneComponent.K2_GetComponentLocation` (`self.Cube`)))))

(event `self.Box1.OnComponentBeginOverlap`
  (params (OverlappedComponent :type "PrimitiveComponent Object Reference") (OtherActor :type "Actor Object Reference") (OtherComp :type "PrimitiveComponent Object Reference") (OtherBodyIndex :type Integer) (bFromSweep :type Boolean) (SweepResult :type "HitResult Structure (by ref)"))
  (bind (_direction `_新規track_0`) (`Timeline|タイムライン_0` :!label _label)
    (:`Update`
      (bind _output_get (set `self.NowPosition` (`KismetMathLibrary.MakeVector` (.x (stale `self.ReceiveBeginPlay` _output_get)) (.y (stale `self.ReceiveBeginPlay` _output_get)) (+ (.z (stale `self.ReceiveBeginPlay` _output_get)) `_新規track_0`))))
      (`SceneComponent.K2_SetWorldLocation` (`self.Cube`) _output_get false false))))

(event `self.Box1.OnComponentEndOverlap`
  (params (OverlappedComponent :type "PrimitiveComponent Object Reference") (OtherActor :type "Actor Object Reference") (OtherComp :type "PrimitiveComponent Object Reference") (OtherBodyIndex :type Integer))
  (goto _label :!via `Stop`))

(fn `UserConstructionScript`)