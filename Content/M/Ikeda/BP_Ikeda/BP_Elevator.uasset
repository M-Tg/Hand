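; Elevator actor that moves its Cube vertically between the start height and a raised height when something enters the Ride trigger.
; Timeline TlUp drives the Z offset from the BeginPlay position, playing forward to rise and in reverse to descend.
; A Moving flag blocks retriggering mid-travel, and finishing flips the UP/Down flags for the next ride.
; Leaving the trigger does not stop travel; Tick and several disconnected older movement graphs do nothing.
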(event `self.ReceiveBeginPlay`
  (bind _output_get (set `self.startPotision` (`SceneComponent.K2_GetComponentLocation` (`self.Cube`))))
  (set `self.NowPosition` _output_get))

(event `self.ReceiveTick`
  (params (DeltaSeconds :type "Float (single-precision)"))
  (if (`self.Moving`)
    _))

(event `self.Ride.OnComponentBeginOverlap`
  (params (OverlappedComponent :type "PrimitiveComponent Object Reference") (OtherActor :type "Actor Object Reference") (OtherComp :type "PrimitiveComponent Object Reference") (OtherBodyIndex :type Integer) (bFromSweep :type Boolean) (SweepResult :type "HitResult Structure (by ref)"))
  (if (not (`self.Moving`))
    (set `self.Moving` true)
    (if (`self.UP`)
      (bind (_direction _z) (`Timeline|tl Up` :!via `PlayFromStart` :!label _label)
        (:`Update`
          (bind _returnvalue (`KismetMathLibrary.MakeVector` (.x (`self.startPotision`)) (.y (`self.startPotision`)) (+ (.z (`self.startPotision`)) _z)))
          (set `self.NowPosition` _returnvalue)
          (`SceneComponent.K2_SetWorldLocation` (`self.Cube`) (`self.NowPosition`) false false :!label _label_2))
        (:`Finished`
          (set `self.NowPosition` _returnvalue)
          (set `self.Moving` false)
          (if (`self.UP`)
            (set `self.UP` false)
            (set `self.Down` true)
            (goto _label_2)
            (elif (`self.Down`)
              (set `self.UP` true)
              (set `self.Down` false)
              (goto _label_2)))))
      (elif (`self.Down`)
        (goto _label :!via `ReverseFromEnd`)))))

(event `self.Ride.OnComponentEndOverlap`
  (params (OverlappedComponent :type "PrimitiveComponent Object Reference") (OtherActor :type "Actor Object Reference") (OtherComp :type "PrimitiveComponent Object Reference") (OtherBodyIndex :type Integer)))

(fn `UserConstructionScript`)