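; BP_Warp is a two-way teleporter that moves any actor overlapping one of its boxes, BoxA or BoxB, to the other box's location.
; Each warp spawns an emitter at the destination.
; A flag per direction blocks an immediate bounce back, and it clears when an overlap ends on the destination box.
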(event `self.BoxA.OnComponentBeginOverlap`
  (params (OverlappedComponent :type "PrimitiveComponent Object Reference") (OtherActor :type "Actor Object Reference") (OtherComp :type "PrimitiveComponent Object Reference") (OtherBodyIndex :type Integer) (bFromSweep :type Boolean) (SweepResult :type "HitResult Structure (by ref)"))
  (bind _returnvalue (`SceneComponent.K2_GetComponentLocation` (`self.BoxB`)))
  (if (not (`self.isWarpfromB`))
    (set `self.isWarpfromA` true)
    (`self.K2_SetActorLocation` OtherActor _returnvalue false false)
    (`GameplayStatics.SpawnEmitterAtLocation` null _returnvalue)))

(event `self.BoxA.OnComponentEndOverlap`
  (params (OverlappedComponent :type "PrimitiveComponent Object Reference") (OtherActor :type "Actor Object Reference") (OtherComp :type "PrimitiveComponent Object Reference") (OtherBodyIndex :type Integer))
  (set `self.isWarpfromB` false))

(event `self.BoxB.OnComponentBeginOverlap`
  (params (OverlappedComponent :type "PrimitiveComponent Object Reference") (OtherActor :type "Actor Object Reference") (OtherComp :type "PrimitiveComponent Object Reference") (OtherBodyIndex :type Integer) (bFromSweep :type Boolean) (SweepResult :type "HitResult Structure (by ref)"))
  (bind _returnvalue (`SceneComponent.K2_GetComponentLocation` (`self.BoxA`)))
  (if (not (`self.isWarpfromA`))
    (set `self.isWarpfromB` true)
    (`self.K2_SetActorLocation` OtherActor _returnvalue false false)
    (`GameplayStatics.SpawnEmitterAtLocation` null _returnvalue)))

(event `self.BoxB.OnComponentEndOverlap`
  (params (OverlappedComponent :type "PrimitiveComponent Object Reference") (OtherActor :type "Actor Object Reference") (OtherComp :type "PrimitiveComponent Object Reference") (OtherBodyIndex :type Integer))
  (set `self.isWarpfromA` false))

(fn `UserConstructionScript`)