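; BP_Goal2 is a stage goal actor that triggers level completion when anything overlaps its Sphere component.
; On overlap it sets IsClear from Success and copies the game mode's Time into BP_GameInstance.
; It then unbinds all destroyed-event handlers on the player pawn and passes the current level name to the game mode's StageClearMessage.
; A direct jump to the "End" level remains in the graph but is disconnected.
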(event `self.Sphere.OnComponentBeginOverlap`
  (params (OverlappedComponent :type "PrimitiveComponent Object Reference") (OtherActor :type "Actor Object Reference") (OtherComp :type "PrimitiveComponent Object Reference") (OtherBodyIndex :type Integer) (bFromSweep :type Boolean) (SweepResult :type "HitResult Structure (by ref)"))
  (bind (_asbp_game_instance _bsuccess) (cast `/Game/M/Mori/BP/BP_GameInstance` (`GameplayStatics.GetGameInstance`) :!pure true))
  ;[1 1 1] ゲームインスタンスをマップ＆モードで選択したらもう一度繋ぎなおす　純粋Cast,Set
  (set `/Game/M/Mori/BP/BP_GameInstance.IsClear` _bsuccess _asbp_game_instance)
  (set `/Game/M/Mori/BP/BP_GameInstance.Time` (`/Game/M/Mori/BP/BP_GameMode.Time` (cast `/Game/M/Mori/BP/BP_GameMode` (`GameplayStatics.GetGameMode`) :!pure true)) _asbp_game_instance)
  (clear `self.OnDestroyed` (`GameplayStatics.GetPlayerPawn` 0))
  (bind _returnvalue (`GameplayStatics.GetCurrentLevelName` true))
  (message `/Game/M/Mori/BP/BP_Interface.Stage Clear` (`GameplayStatics.GetGameMode`) (`KismetStringLibrary.Conv_StringToName` _returnvalue)))

(fn `UserConstructionScript`)