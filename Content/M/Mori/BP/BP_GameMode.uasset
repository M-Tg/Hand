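; Game mode that runs stage flow for switch-and-gate levels, covering gate signals, level progression and player respawn.
; Interface events store the required switch count, relay active state as gate open/close dispatcher calls, and load Proto2 after Proto1 or End otherwise.
; A looping timer counts elapsed seconds.
; Pawn destruction restarts the player, flags Restart on BP_GameInstance and re-runs the OnDestroyed binding for the new pawn.
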(event `/Game/M/Mori/BP/BP_Interface.Required Number Of Switches`
  (params (`Required Switch` :type Integer))
  ;[1 1 1] Interface
  (set `self.Required Switch` `Required Switch`))

(event `/Game/M/Mori/BP/BP_Interface.Active State`
  (params (IsActive :type Boolean))
  ;[1 1 1] Interface
  (if IsActive
    (`self.GateOpen_EventDispatcuer`)
    (else
      (`self.GateClose_EventDispatcuer`))))

(event `/Game/M/Mori/BP/BP_Interface.Stage Clear`
  (params (`Clear Stage Name` :type Name))
  ;[1 1 1] Interface
  (if (== `Clear Stage Name` "Proto1")
    (`GameplayStatics.OpenLevel` "Proto2")
    (else
      (if (== `Clear Stage Name` "Proto2")
        _
        (else
          _))
      (`GameplayStatics.OpenLevel` "End"))))

(event `self.ReceiveBeginPlay`
  (`self.TimeEvent`)
  (`self.RestartEvent`))

(event `TimeEvent`
  ;[1 1 1] Time Count
  (`KismetSystemLibrary.K2_SetTimerDelegate` (delegate `Count`) 1.0 true))

(event `RestartEvent`
  (bind _returnvalue (`GameplayStatics.GetPlayerPawn` 0))
  ;[1 1 1] Restart
  (if (!= _returnvalue null)
    (add `self.OnDestroyed` _returnvalue (delegate `RestartPlayerEvent`))
    (`KismetSystemLibrary.PrintString` "Death")
    (else
      (`KismetSystemLibrary.PrintString` "Restart"))))

(event `RestartPlayerEvent` :!signature `self.OnDestroyed`
  (params (DestroyedActor :type "Actor Object Reference"))
  ;[1 1 1] Restart
  (`self.RestartPlayer` (`GameplayStatics.GetPlayerController` 0))
  (set `/Game/M/Mori/BP/BP_GameInstance.Restart` true (cast `/Game/M/Mori/BP/BP_GameInstance` (`GameplayStatics.GetGameInstance`) :!pure true))
  (`self.RestartEvent`))

(event `Count`
  ;[1 1 1] Time Count
  (set `self.Time` (+ (`self.Time`) 1)))

(fn `UserConstructionScript`)