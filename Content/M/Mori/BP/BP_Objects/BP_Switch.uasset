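; BP_Switch is a switch actor that animates its Cylinder's height when something enters or leaves its Sphere trigger.
; Begin and end overlap each play their own timeline from the start, setting the Cylinder's relative Z to the track value plus a fixed offset.
; Overlaps are not filtered by actor, both updates print debug strings, and no other object is notified.
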(event `self.Sphere.OnComponentBeginOverlap`
  (params (OverlappedComponent :type "PrimitiveComponent Object Reference") (OtherActor :type "Actor Object Reference") (OtherComp :type "PrimitiveComponent Object Reference") (OtherBodyIndex :type Integer) (bFromSweep :type Boolean) (SweepResult :type "HitResult Structure (by ref)"))
  (bind (_direction `_新規track_0`) (`Timeline|TimeLine` :!via `PlayFromStart`)
    (:`Update`
      (`KismetSystemLibrary.PrintString` "pppp")
      (`SceneComponent.K2_SetRelativeLocation` (`self.Cylinder`) (`KismetMathLibrary.MakeVector` 0.0 0.0 (+ `_新規track_0` 15.0)) false false))))

(event `self.Sphere.OnComponentEndOverlap`
  (params (OverlappedComponent :type "PrimitiveComponent Object Reference") (OtherActor :type "Actor Object Reference") (OtherComp :type "PrimitiveComponent Object Reference") (OtherBodyIndex :type Integer))
  (bind (_direction `_新規track_0`) (`Timeline|タイムライン_0` :!via `PlayFromStart`)
    (:`Update`
      (`KismetSystemLibrary.PrintString` "q")
      (`SceneComponent.K2_SetRelativeLocation` (`self.Cylinder`) (`KismetMathLibrary.MakeVector` 0.0 0.0 (+ `_新規track_0` 15.0)) false false))))

(fn `UserConstructionScript`)