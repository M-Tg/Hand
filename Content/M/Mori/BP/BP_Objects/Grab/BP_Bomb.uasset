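; BP_Bomb is a bomb object that explodes when it registers a hit while moving.
; Each Tick, while Hit is true, it requires the Sphere's physics velocity to be non-negligible on both Y and Z, ignoring X.
; It then spawns EffectActor_explosion at the Sphere's relative transform, destroys itself and prints a debug string.
; The construction script applies a corrugated metal material to the Sphere.
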(event `self.ReceiveBeginPlay`
  (`parent.ReceiveBeginPlay`))

(event `self.ReceiveTick`
  (params (DeltaSeconds :type "Float (single-precision)"))
  (`parent.ReceiveTick` DeltaSeconds)
  (if (`self.Hit`)
    (bind _returnvalue (`PrimitiveComponent.GetPhysicsLinearVelocity` (`self.Sphere`) "None"))
    (set `self.VelocityY` (.y _returnvalue))
    (set `self.VelocityZ` (.z _returnvalue))
    (if (and (or (> (`self.VelocityY`) 0.1) (< (`self.VelocityY`) -0.1)) (or (> (`self.VelocityZ`) 0.1) (< (`self.VelocityZ`) -0.1)))
      (`|SpawnActorFromClass` "/Game/M/Mori/BP/BP_Objects/Grab/EffectActor_explosion.EffectActor_explosion_C" (`SceneComponent.GetRelativeTransform` (`self.Sphere`)) "Undefined" "OverrideRootScale" null null)
      (`self.K2_DestroyActor`)
      (`KismetSystemLibrary.PrintString` "Bomb"))))

(fn `UserConstructionScript`
  (`parent.UserConstructionScript`)
  (`PrimitiveComponent.SetMaterial` (`self.Sphere`) 0 "/Game/MS_InMetalEss/Surface/02_Corrugated_Metal_Sheet_2x2_M_tdhnebok/02_Corrugated_Metal_Sheet_2x2_M_tdhnebok_8K_inst.02_Corrugated_Metal_Sheet_2x2_M_tdhnebok_8K_inst"))