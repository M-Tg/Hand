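; Grabbable breakable ball that tracks whether it is grounded and free to be grabbed, showing that state through its colour.
; Until Break is set, Tick moves NoCollision to the Sphere's location and toggles collision on Up and Down to refresh overlaps.
; Up overlaps block grabbing and Down overlaps mean grounded.
; A construction-script dynamic material shows cyan for grabbable, red for blocked, yellow for not grounded.
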(event `CollisionCheck`
  (params (Collision :type "PrimitiveComponent Object Reference"))
  (`PrimitiveComponent.SetCollisionEnabled` Collision "NoCollision")
  (`PrimitiveComponent.SetCollisionEnabled` Collision "QueryOnly"))

(event `self.ReceiveTick`
  (params (DeltaSeconds :type "Float (single-precision)"))
  (if (not (`self.Break`))
    ;[1 1 1] Range location
    (`SceneComponent.K2_SetWorldLocation` (`self.NoCollision`) (`SceneComponent.K2_GetComponentLocation` (`self.Sphere`)) false false)
    (`self.CollisionCheck` (`self.Up`))
    (`self.CollisionCheck` (`self.Down`))
    (if (`self.Grounded`)
      (if (`self.CanBeGrabed`)
        (`MaterialInstanceDynamic.SetVectorParameterValue` (`self.SphereMaterial`) "SampleColor" (struct :`R` 0.283715 :`G` 0.797356 :`B` 0.916667 :`A` 1.0))
        (else
          (`MaterialInstanceDynamic.SetVectorParameterValue` (`self.SphereMaterial`) "SampleColor" (struct :`R` 0.916667 :`G` 0.131587 :`B` 0.186345 :`A` 1.0))))
      (else
        (`MaterialInstanceDynamic.SetVectorParameterValue` (`self.SphereMaterial`) "SampleColor" (struct :`R` 0.916667 :`G` 0.754615 :`B` 0.139466 :`A` 1.0))))))

(event `self.Up.OnComponentBeginOverlap`
  (params (OverlappedComponent :type "PrimitiveComponent Object Reference") (OtherActor :type "Actor Object Reference") (OtherComp :type "PrimitiveComponent Object Reference") (OtherBodyIndex :type Integer) (bFromSweep :type Boolean) (SweepResult :type "HitResult Structure (by ref)"))
  (set `self.CanBeGrabed` false))

(event `self.Up.OnComponentEndOverlap`
  (params (OverlappedComponent :type "PrimitiveComponent Object Reference") (OtherActor :type "Actor Object Reference") (OtherComp :type "PrimitiveComponent Object Reference") (OtherBodyIndex :type Integer))
  (set `self.CanBeGrabed` true))

(event `self.Down.OnComponentBeginOverlap`
  (params (OverlappedComponent :type "PrimitiveComponent Object Reference") (OtherActor :type "Actor Object Reference") (OtherComp :type "PrimitiveComponent Object Reference") (OtherBodyIndex :type Integer) (bFromSweep :type Boolean) (SweepResult :type "HitResult Structure (by ref)"))
  (set `self.Grounded` true))

(event `self.SphereRange.OnComponentBeginOverlap`
  (params (OverlappedComponent :type "PrimitiveComponent Object Reference") (OtherActor :type "Actor Object Reference") (OtherComp :type "PrimitiveComponent Object Reference") (OtherBodyIndex :type Integer) (bFromSweep :type Boolean) (SweepResult :type "HitResult Structure (by ref)")))

(event `self.Down.OnComponentEndOverlap`
  (params (OverlappedComponent :type "PrimitiveComponent Object Reference") (OtherActor :type "Actor Object Reference") (OtherComp :type "PrimitiveComponent Object Reference") (OtherBodyIndex :type Integer))
  (set `self.Grounded` false))

(event `self.SphereRange.OnComponentEndOverlap`
  (params (OverlappedComponent :type "PrimitiveComponent Object Reference") (OtherActor :type "Actor Object Reference") (OtherComp :type "PrimitiveComponent Object Reference") (OtherBodyIndex :type Integer)))

(fn `UserConstructionScript`
  ;[1 1 1] マテリアルをダイナミックインスタンス化　選んだ親マテリアルをベースにメッシュ用のマテリアル作成
  (bind _returnvalue (`KismetMaterialLibrary.CreateDynamicMaterialInstance` "/Game/M/Mori/BP/BP_Objects/SampleMaterial.SampleMaterial" "SampleMaterial"))
  (bind _output_get (set `self.SphereMaterial` _returnvalue))
  (`PrimitiveComponent.SetMaterial` (`self.Sphere`) 0 _output_get)
  (`MaterialInstanceDynamic.SetVectorParameterValue` _output_get "SampleColor" (struct :`R` 0.283715 :`G` 0.797356 :`B` 0.916667 :`A` 1.0)))