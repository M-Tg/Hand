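; BP_Needle is a needle hazard that deals heavy damage to BP_Player when it overlaps the KillRabge volume.
; The construction script gives the Cube a dynamic material, tinted blue by default.
; Tick toggles KillRabge collision off and back to query-only to re-evaluate overlaps each frame.
; Overlap begin and end set a Hit flag for any actor, which Tick uses to switch the cube between red and blue.
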(event `CollisionCheck`
  (params (Collision :type "PrimitiveComponent Object Reference"))
  (`PrimitiveComponent.SetCollisionEnabled` Collision "NoCollision")
  (`PrimitiveComponent.SetCollisionEnabled` Collision "QueryOnly"))

(event `self.ReceiveTick`
  (params (DeltaSeconds :type "Float (single-precision)"))
  (`self.CollisionCheck` (`self.Kill Rabge`))
  (if (`self.Hit`)
    (`MaterialInstanceDynamic.SetVectorParameterValue` (`self.Cube Material`) "SampleColor" (struct :`R` 0.916667 :`G` 0.131587 :`B` 0.186345 :`A` 1.0))
    (else
      (`MaterialInstanceDynamic.SetVectorParameterValue` (`self.Cube Material`) "SampleColor" (struct :`R` 0.283715 :`G` 0.797356 :`B` 0.916667 :`A` 1.0)))))

(event `self.Kill Rabge.OnComponentBeginOverlap`
  (params (OverlappedComponent :type "PrimitiveComponent Object Reference") (OtherActor :type "Actor Object Reference") (OtherComp :type "PrimitiveComponent Object Reference") (OtherBodyIndex :type Integer) (bFromSweep :type Boolean) (SweepResult :type "HitResult Structure (by ref)"))
  (set `self.Hit` true)
  (bind _asbp_player (cast `/Game/M/Mori/BP/Player/BP_Player` OtherActor))
  (`GameplayStatics.ApplyDamage` _asbp_player 100.0))

(event `self.Kill Rabge.OnComponentEndOverlap`
  (params (OverlappedComponent :type "PrimitiveComponent Object Reference") (OtherActor :type "Actor Object Reference") (OtherComp :type "PrimitiveComponent Object Reference") (OtherBodyIndex :type Integer))
  (set `self.Hit` false))

(fn `UserConstructionScript`
  ;[1 1 1] マテリアルをダイナミックインスタンス化　選んだ親マテリアルをベースにメッシュ用のマテリアル作成
  (bind _returnvalue (`KismetMaterialLibrary.CreateDynamicMaterialInstance` "/Game/M/Mori/BP/BP_Objects/SampleMaterial.SampleMaterial" "SampleMaterial"))
  (bind _output_get (set `self.Cube Material` _returnvalue))
  (`PrimitiveComponent.SetMaterial` (`self.Cube`) 0 _output_get)
  (`MaterialInstanceDynamic.SetVectorParameterValue` _output_get "SampleColor" (struct :`R` 0.283715 :`G` 0.797356 :`B` 0.916667 :`A` 1.0)))