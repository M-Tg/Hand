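; BP_Press is a static-object Blueprint for a press whose cylinder moves back and forth continuously along its local Z axis.
; Each Tick adds or subtracts Speed from Length and sets the cylinder's relative Z location to that value.
; The Way boolean flips at MaxLength and at zero to reverse direction.
; The step ignores delta time, so the motion rate depends on frame rate.
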(event `self.ReceiveTick`
  (params (DeltaSeconds :type "Float (single-precision)"))
  (if (`self.Way`)
    (set `self.length` (+ (`self.length`) (`self.Speed`)))
    (`SceneComponent.K2_SetRelativeLocation` (`self.Shape_Cylinder`) (`KismetMathLibrary.MakeVector` 0.0 0.0 (`self.length`)) false false)
    (if (>= (`self.length`) (`self.Max Length`))
      (set `self.Way` false))
    (else
      (set `self.length` (- (`self.length`) (`self.Speed`)))
      (`SceneComponent.K2_SetRelativeLocation` (`self.Shape_Cylinder`) (`KismetMathLibrary.MakeVector` 0.0 0.0 (`self.length`)) false false)
      (if (>= 0.0 (`self.length`))
        (set `self.Way` true)))))

(fn `UserConstructionScript`)