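; BP_FireWall is a fire wall obstacle that shuts off while a BP_Plug that overlapped its Plug collision is stationary.
; Tick toggles the Plug collision off and on to refresh overlaps, then reads the stored actor's Moving state.
; Stopping sets FireCollision to ignore Pawns and plays the FireScale timeline to scale the flamethrower effect.
; A moving or absent plug restores Pawn blocking and reverses the timeline.
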(event `self.Plug.OnComponentBeginOverlap`
  (params (OverlappedComponent :type "PrimitiveComponent Object Reference") (OtherActor :type "Actor Object Reference") (OtherComp :type "PrimitiveComponent Object Reference") (OtherBodyIndex :type Integer) (bFromSweep :type Boolean) (SweepResult :type "HitResult Structure (by ref)"))
  (set `self.Plug Actor` OtherActor))

(event `CollisionCheck`
  (params (Collision :type "PrimitiveComponent Object Reference"))
  (`PrimitiveComponent.SetCollisionEnabled` Collision "NoCollision")
  (`PrimitiveComponent.SetCollisionEnabled` Collision "QueryOnly"))

(event `self.ReceiveTick`
  (params (DeltaSeconds :type "Float (single-precision)"))
  (`self.CollisionCheck` (`self.Plug`))
  (bind _asbp_plug (cast `/Game/M/Mori/BP/BP_Objects/Static/fire/BP_Plug` (`self.Plug Actor`))
    (:`then`
      (if (`/Game/M/Mori/BP/BP_Objects/Static/fire/BP_Plug.Moving` _asbp_plug)
        (if (`self.Stop`) :!label _label
          (`self.StartFire`))
        (elif (not (`self.Stop`))
          (`self.StopFire`))))
    (:`CastFailed`
      (goto _label))))

(event `StopFire`
  (set `self.Stop` true)
  (`PrimitiveComponent.SetCollisionResponseToChannel` (`self.Fire Collision`) "ECC_Pawn" "ECR_Ignore")
  (bind (_direction `_新規track_1`) (`Timeline|FireScale` :!via `PlayFromStart` :!label _label_2)
    (:`Update`
      (`SceneComponent.SetWorldScale3D` (`self.P_Flamethrower`) (`KismetMathLibrary.MakeVector` `_新規track_1` `_新規track_1` `_新規track_1`)))))

(event `StartFire`
  (set `self.Stop` false)
  (`PrimitiveComponent.SetCollisionResponseToChannel` (`self.Fire Collision`) "ECC_Pawn" "ECR_Block")
  (goto _label_2 :!via `ReverseFromEnd`))

(fn `UserConstructionScript`)