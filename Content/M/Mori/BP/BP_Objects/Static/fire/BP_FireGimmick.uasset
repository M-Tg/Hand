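; BP_FireGimmick is a fire puzzle object that turns an associated BP_Plug when something overlaps its PlayerSide collision.
; FireSide and PlugSide overlaps register the fire and plug actors, and PlayerSide calls TurnPlug on the stored plug.
; Tick toggles collision off and on for FireSide and PlugSide to refresh overlap detection every frame.
; Calls to start or stop BP_FireWall and to return the plug are unwired.
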(event `self.FireSide.OnComponentBeginOverlap`
  (params (OverlappedComponent :type "PrimitiveComponent Object Reference") (OtherActor :type "Actor Object Reference") (OtherComp :type "PrimitiveComponent Object Reference") (OtherBodyIndex :type Integer) (bFromSweep :type Boolean) (SweepResult :type "HitResult Structure (by ref)"))
  ;[1 1 1] レーバーと炎のアクタの登録
  (set `self.Fire Actor` OtherActor))

(event `self.ReceiveTick`
  (params (DeltaSeconds :type "Float (single-precision)"))
  (`self.CollisionCheck` (`self.FireSide`))
  (`self.CollisionCheck` (`self.PlugSide`)))

(event `self.PlugSide.OnComponentBeginOverlap`
  (params (OverlappedComponent :type "PrimitiveComponent Object Reference") (OtherActor :type "Actor Object Reference") (OtherComp :type "PrimitiveComponent Object Reference") (OtherBodyIndex :type Integer) (bFromSweep :type Boolean) (SweepResult :type "HitResult Structure (by ref)"))
  ;[1 1 1] レーバーと炎のアクタの登録
  (set `self.Plug Actor` OtherActor))

(event `CollisionCheck`
  (params (Collision :type "PrimitiveComponent Object Reference"))
  (`PrimitiveComponent.SetCollisionEnabled` Collision "NoCollision")
  (`PrimitiveComponent.SetCollisionEnabled` Collision "QueryOnly"))

(event `self.PlayerSide.OnComponentBeginOverlap`
  (params (OverlappedComponent :type "PrimitiveComponent Object Reference") (OtherActor :type "Actor Object Reference") (OtherComp :type "PrimitiveComponent Object Reference") (OtherBodyIndex :type Integer) (bFromSweep :type Boolean) (SweepResult :type "HitResult Structure (by ref)"))
  (bind (_asbp_plug _bsuccess) (cast `/Game/M/Mori/BP/BP_Objects/Static/fire/BP_Plug` (`self.Plug Actor`) :!pure true))
  ;[1 1 1] Plugの操作
  (if _bsuccess
    (`/Game/M/Mori/BP/BP_Objects/Static/fire/BP_Plug.Turn Plug` _asbp_plug)))

(event `self.PlayerSide.OnComponentEndOverlap`
  (params (OverlappedComponent :type "PrimitiveComponent Object Reference") (OtherActor :type "Actor Object Reference") (OtherComp :type "PrimitiveComponent Object Reference") (OtherBodyIndex :type Integer)))

(fn `UserConstructionScript`)