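; BP_Switch is a switch that activates while an actor overlaps its Sphere, apparently to drive a door.
; Begin and end overlap set IsActive; the player-only check is disconnected.
; Tick toggles Sphere collision off and on to refresh overlaps, then plays or reverses a timeline from IsActive.
; Timeline updates move the Cylinder vertically and send IsActive to the GameMode through an interface message.
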(event `self.ReceiveTick`
  (params (DeltaSeconds :type "Float (single-precision)"))
  (`self.CollisionCheck` (`self.Sphere`))
  (if (`self.Is Active`)
    (bind (_direction `_新規track_0`) (`Timeline|TimeLine` :`NewTime` 0.0 :!label _label)
      (:`Update`
        (`SceneComponent.K2_SetRelativeLocation` (`self.Cylinder`) (`KismetMathLibrary.MakeVector` 0.0 0.0 (+ `_新規track_0` 15.0)) false false)
        ;[1 1 1] Interface & Door
        (message `/Game/M/Mori/BP/BP_Interface.Active State` (`GameplayStatics.GetGameMode`) (`self.Is Active`))))
    (else
      (goto _label :!via `Reverse`))))

(event `CollisionCheck`
  (params (Collision :type "PrimitiveComponent Object Reference"))
  (`PrimitiveComponent.SetCollisionEnabled` Collision "NoCollision")
  (`PrimitiveComponent.SetCollisionEnabled` Collision "QueryOnly"))

(event `self.Sphere.OnComponentBeginOverlap`
  (params (OverlappedComponent :type "PrimitiveComponent Object Reference") (OtherActor :type "Actor Object Reference") (OtherComp :type "PrimitiveComponent Object Reference") (OtherBodyIndex :type Integer) (bFromSweep :type Boolean) (SweepResult :type "HitResult Structure (by ref)"))
  (set `self.Is Active` true))

(event `self.Sphere.OnComponentEndOverlap`
  (params (OverlappedComponent :type "PrimitiveComponent Object Reference") (OtherActor :type "Actor Object Reference") (OtherComp :type "PrimitiveComponent Object Reference") (OtherBodyIndex :type Integer))
  (set `self.Is Active` false))

(fn `UserConstructionScript`)