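; BP_Gate is a switch-driven gate whose Cube slides vertically relative to its Cylinder.
; On BeginPlay it sends its required switch count to the game mode through an interface and binds to BP_GameMode's open and close dispatchers.
; Each dispatcher call moves the Cube one fixed step, so full travel takes repeated calls.
; Travel limits come from the starting Z offset to the Cylinder and its negation.
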(event `self.ReceiveBeginPlay`
  (bind _output_get (set `self.MinZ` (- (.z (`SceneComponent.K2_GetComponentLocation` (`self.Cube`))) (.z (`SceneComponent.K2_GetComponentLocation` (`self.Cylinder`))))))
  (set `self.MaxZ` (* _output_get -1.0))
  ;[1 1 1] Interface で必要スイッチ数を管理
  (message `/Game/M/Mori/BP/System/BP_Interface.Required Number Of Switches` (`GameplayStatics.GetGameMode`) (`self.Number Of Required`))
  (bind _asbp_game_mode (cast `/Game/M/Mori/BP/System/BP_GameMode` (`GameplayStatics.GetGameMode`)))
  (add `/Game/M/Mori/BP/System/BP_GameMode.GateOpen_EventDispatcuer` _asbp_game_mode (delegate `Open Gate`))
  (add `/Game/M/Mori/BP/System/BP_GameMode.GateClose_EventDispatcuer` _asbp_game_mode (delegate `Close Gate`)))

(event `self.ReceiveTick`
  (params (DeltaSeconds :type "Float (single-precision)")))

(event `Open Gate`
  (bind _cube (`self.Cube`))
  (bind (_returnvalue_x _returnvalue_y _returnvalue_z) (`KismetMathLibrary.BreakVector` (`SceneComponent.K2_GetComponentLocation` _cube)))
  (bind (_returnvalue_x_2 _returnvalue_y_2 _returnvalue_z_2) (`KismetMathLibrary.BreakVector` (`SceneComponent.K2_GetComponentLocation` (`self.Cylinder`))))
  (if (< (- _returnvalue_z _returnvalue_z_2) (`self.MaxZ`))
    (`SceneComponent.K2_SetWorldLocation` _cube (`KismetMathLibrary.MakeVector` _returnvalue_x _returnvalue_y (+ _returnvalue_z 10.0)) false false)))

(event `Close Gate`
  (bind _cube (`self.Cube`))
  (bind (_returnvalue_x _returnvalue_y _returnvalue_z) (`KismetMathLibrary.BreakVector` (`SceneComponent.K2_GetComponentLocation` _cube)))
  (bind (_returnvalue_x_2 _returnvalue_y_2 _returnvalue_z_2) (`KismetMathLibrary.BreakVector` (`SceneComponent.K2_GetComponentLocation` (`self.Cylinder`))))
  (if (> (- _returnvalue_z _returnvalue_z_2) (`self.MinZ`))
    (`SceneComponent.K2_SetWorldLocation` _cube (`KismetMathLibrary.MakeVector` _returnvalue_x _returnvalue_y (+ _returnvalue_z -10.0)) false false)))

(fn `UserConstructionScript`)