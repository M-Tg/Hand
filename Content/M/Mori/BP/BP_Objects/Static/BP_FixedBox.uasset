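; BP_FixedBox is a static box object that tracks whether it can be climbed on its left and right sides.
; Overlaps on the UpLSide and UpRSide collision components set CanBeClimbedL and CanBeClimbedR false when they begin and true when they end.
; Every Tick, CollisionCheck switches both components to NoCollision and back to QueryOnly, forcing overlaps to be re-evaluated each frame.
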(event `CollisionCheck`
  (params (Collision :type "PrimitiveComponent Object Reference"))
  (`PrimitiveComponent.SetCollisionEnabled` Collision "NoCollision")
  (`PrimitiveComponent.SetCollisionEnabled` Collision "QueryOnly"))

(event `self.ReceiveActorBeginOverlap`
  (params (OtherActor :type "Actor Object Reference")))

(event `self.UpLSide.OnComponentBeginOverlap`
  (params (OverlappedComponent :type "PrimitiveComponent Object Reference") (OtherActor :type "Actor Object Reference") (OtherComp :type "PrimitiveComponent Object Reference") (OtherBodyIndex :type Integer) (bFromSweep :type Boolean) (SweepResult :type "HitResult Structure (by ref)"))
  (set `self.CanBeClimbedL` false))

(event `self.UpRSide.OnComponentBeginOverlap`
  (params (OverlappedComponent :type "PrimitiveComponent Object Reference") (OtherActor :type "Actor Object Reference") (OtherComp :type "PrimitiveComponent Object Reference") (OtherBodyIndex :type Integer) (bFromSweep :type Boolean) (SweepResult :type "HitResult Structure (by ref)"))
  (set `self.CanBeClimbedR` false))

(event `self.ReceiveTick`
  (params (DeltaSeconds :type "Float (single-precision)"))
  (`self.CollisionCheck` (`self.UpLSide`))
  (`self.CollisionCheck` (`self.UpRSide`)))

(event `self.UpLSide.OnComponentEndOverlap`
  (params (OverlappedComponent :type "PrimitiveComponent Object Reference") (OtherActor :type "Actor Object Reference") (OtherComp :type "PrimitiveComponent Object Reference") (OtherBodyIndex :type Integer))
  (set `self.CanBeClimbedL` true))

(event `self.UpRSide.OnComponentEndOverlap`
  (params (OverlappedComponent :type "PrimitiveComponent Object Reference") (OtherActor :type "Actor Object Reference") (OtherComp :type "PrimitiveComponent Object Reference") (OtherBodyIndex :type Integer))
  (set `self.CanBeClimbedR` true))

(fn `UserConstructionScript`)