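; Game mode that runs stage flow: switch-gate signals, player respawn, stage clearing and level progression.
; Interface events store the required switch count, relay active state to gate open/close dispatchers, and start the clear fade.
; Tick watches the GameInstance clear flag, counts down, then opens the next Proto level or End by stage name.
; A pawn-destroyed binding respawns the player and rebinds; separate events count seconds, reload the level, or swap streamed stages.
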(event `Next Stage`
  (`GameplayStatics.UnloadStreamLevelBySoftObjectPtr` "/Game/M/Mori/Map/Stage1.Stage1")
  (`GameplayStatics.LoadStreamLevelBySoftObjectPtr` "/Game/M/Mori/Map/Stage2.Stage2" true true)
  (`self.K2_SetActorTransform` (`GameplayStatics.GetPlayerPawn` 0) (`self.GetTransform` (`self.K2_FindPlayerStart` null)) false false))

(event `Restart`
  (bind _returnvalue (`GameplayStatics.GetCurrentLevelName` true))
  (`GameplayStatics.OpenLevel` (`KismetStringLibrary.Conv_StringToName` _returnvalue)))

(event `/Game/M/Mori/BP/System/BP_Interface.Required Number Of Switches`
  (params (`Required Switch` :type Integer))
  ;[1 1 1] Interface
  (set `self.Required Switch` `Required Switch`))

(event `/Game/M/Mori/BP/System/BP_Interface.Stage Clear`
  (params (`Clear Stage Name` :type Name))
  ;[1 1 1] Interface
  (`PlayerCameraManager.StartCameraFade` :`self` (`GameplayStatics.GetPlayerCameraManager` 0) :`ToAlpha` 1.0 :`Duration` 1.0 :`bHoldWhenFinished` true)
  (set `/Game/M/Mori/BP/System/BP_GameInstance.IsClear` true (cast `/Game/M/Mori/BP/System/BP_GameInstance` (`GameplayStatics.GetGameInstance`) :!pure true)))

(event `/Game/M/Mori/BP/System/BP_Interface.Active State`
  (params (IsActive :type Boolean))
  ;[1 1 1] Interface
  (if IsActive
    (`self.GateOpen_EventDispatcuer`)
    (else
      (`self.GateClose_EventDispatcuer`))))

(event `self.ReceiveBeginPlay`
  (`self.TimeEvent`)
  (`self.RestartEvent`)
  (set `self.FadeTime` 2.0)
  (set `/Game/M/Mori/BP/System/BP_GameInstance.IsClear` false (cast `/Game/M/Mori/BP/System/BP_GameInstance` (`GameplayStatics.GetGameInstance`) :!pure true)))

(event `self.ReceiveTick`
  (params (DeltaSeconds :type "Float (single-precision)"))
  (bind _fadetime (`self.FadeTime`))
  ;[1 1 1] Interface
  (if (`/Game/M/Mori/BP/System/BP_GameInstance.IsClear` (cast `/Game/M/Mori/BP/System/BP_GameInstance` (`GameplayStatics.GetGameInstance`) :!pure true))
    (set `self.FadeTime` (- _fadetime DeltaSeconds))
    (if (<= _fadetime 0.0)
      (if (== (stale `/Game/M/Mori/BP/System/BP_Interface.Stage Clear` `Clear Stage Name`) "Proto1")
        (`GameplayStatics.OpenLevel` "Proto2")
        (elif (== (stale `/Game/M/Mori/BP/System/BP_Interface.Stage Clear` `Clear Stage Name`) "Proto2")
          (`GameplayStatics.OpenLevel` "Proto3")
          (else
            (if (== (stale `/Game/M/Mori/BP/System/BP_Interface.Stage Clear` `Clear Stage Name`) "Proto3")
              _
              (else
                _))
            (`GameplayStatics.OpenLevel` "End")))))))

(event `TimeEvent`
  ;[1 1 1] Time Count
  (`KismetSystemLibrary.K2_SetTimerDelegate` (delegate `Count`) 1.0 true))

(event `Count`
  ;[1 1 1] Time Count
  (set `self.Time` (+ (`self.Time`) 1)))

(event `RestartEvent`
  (bind _returnvalue (`GameplayStatics.GetPlayerPawn` 0))
  ;[1 1 1] Restart
  (if (!= _returnvalue null)
    (add `self.OnDestroyed` _returnvalue (delegate `RestartPlayerEvent`))
    (`KismetSystemLibrary.PrintString` "Death")
    (else
      (`KismetSystemLibrary.PrintString` "Restart"))))

(event `RestartPlayerEvent` :!signature `self.OnDestroyed`
  (params (DestroyedActor :type "Actor Object Reference"))
  ;[1 1 1] Restart
  (`self.RestartPlayer` (`GameplayStatics.GetPlayerController` 0))
  (set `/Game/M/Mori/BP/System/BP_GameInstance.Restart` true (cast `/Game/M/Mori/BP/System/BP_GameInstance` (`GameplayStatics.GetGameInstance`) :!pure true))
  (`self.RestartEvent`))

(fn `UserConstructionScript`)