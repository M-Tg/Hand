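; BP_MoveTest is a test actor that shuttles back and forth along the world Y axis.
; Each Tick it offsets its position by a Speed vector without sweep, then flips Speed when its Y location passes either of two fixed bounds.
; The step is per frame rather than scaled by delta time, and an unconnected rotation node never runs.
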(event `self.ReceiveTick`
  (params (DeltaSeconds :type "Float (single-precision)"))
  (bind (_returnvalue_x _returnvalue_y) (`KismetMathLibrary.BreakVector` (`self.K2_GetActorLocation`)))
  (bind (_returnvalue_x_2 _returnvalue_y_2) (`KismetMathLibrary.BreakVector` (`self.K2_GetActorLocation`)))
  (`self.K2_AddActorWorldOffset` (`self.speed`))
  (if (> _returnvalue_y_2 2300.0)
    (set `self.speed` (0.0 -10.0 0.0))
    (elif (< _returnvalue_y 840.0)
      (set `self.speed` (0.0 10.0 0.0)))))

(fn `UserConstructionScript`)