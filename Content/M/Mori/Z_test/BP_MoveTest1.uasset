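; BP_MoveTest1 is a test actor that shuttles back and forth along the world Y axis.
; Each Tick offsets the actor by its Speed vector without sweep, then flips Speed at fixed world-Y limits.
; The step is not scaled by delta time, so travel speed depends on frame rate.
; An incremental rotation node is left unconnected and never runs.
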(event `self.ReceiveTick`
  (params (DeltaSeconds :type "Float (single-precision)"))
  (bind (_returnvalue_x _returnvalue_y) (`KismetMathLibrary.BreakVector` (`self.K2_GetActorLocation`)))
  (bind (_returnvalue_x_2 _returnvalue_y_2) (`KismetMathLibrary.BreakVector` (`self.K2_GetActorLocation`)))
  (`self.K2_AddActorWorldOffset` (`self.speed`))
  (if (> _returnvalue_y_2 0.0)
    (set `self.speed` (0.0 -5.0 0.0))
    (elif (< _returnvalue_y -1200.0)
      (set `self.speed` (0.0 5.0 0.0)))))

(fn `UserConstructionScript`)